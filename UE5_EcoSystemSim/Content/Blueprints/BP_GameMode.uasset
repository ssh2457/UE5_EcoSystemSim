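; Game mode for a plant, hare and fox ecosystem that populates the level and tracks each population.
; BeginPlay caches TriggerVolumes as water pools and TargetPoints as spawn points, then spawns the initial plants and random-sex animals.
; Spawning picks random navigable points within a radius of random spawn points.
; Tick uses a time accumulator to periodically replenish plants below their cap and print population counts; animals are not respawned here.
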(event `self.ReceiveBeginPlay`
  (bind _outactors (`GameplayStatics.GetAllActorsOfClass` "/Script/Engine.TriggerVolume"))
  (set `self.WaterPools` _outactors)
  (bind _outactors_2 (`GameplayStatics.GetAllActorsOfClass` "/Script/Engine.TargetPoint"))
  (set `self.SpawnPoints` _outactors_2)
  (`self.SpawnPlants` 20)
  (`self.SpawnAnimals` "/Game/Blueprints/Animals/Hare/BP_Hare.BP_Hare_C" 50)
  (`self.SpawnAnimals` "/Game/Blueprints/Animals/Fox/BP_Fox.BP_Fox_C" 20))

(event `self.ReceiveTick`
  (params (DeltaSeconds :type "Float (single-precision)"))
  (set `self.cumulatedSeconds` (+ DeltaSeconds (`self.cumulatedSeconds`)))
  (if (>= (`self.cumulatedSeconds`) (`self.SpawnTimeThreshold`))
    (set `self.cumulatedSeconds` (- (`self.cumulatedSeconds`) (`self.SpawnTimeThreshold`)))
    (`|ExecutionSequence`
      (:`then_0`
        (if (< (`BlueprintSetLibrary.Set_Length` (`self.Plants`)) (`self.MaxPlantCount`))
          (`self.SpawnPlants` 20)))
      (:`then_1`
        (`KismetSystemLibrary.PrintText` (`|FormatText` "Plants: {0}" (`BlueprintSetLibrary.Set_Length` (`self.Plants`)))))
      (:`then_2`
        (`KismetSystemLibrary.PrintText` (`|FormatText` "Hares: {0}" (`BlueprintSetLibrary.Set_Length` (`self.Hares`)))))
      (:`then_3`
        (`KismetSystemLibrary.PrintText` (`|FormatText` "Foxes: {0}" (`BlueprintSetLibrary.Set_Length` (`self.Foxes`))))))))

(fn `FindSpawnableLocation`
  (returns (OutSpawnableLocation :type "Vector Structure") (OutFound :type Boolean))
  (bind (_randomlocation _returnvalue) (`NavigationSystemV1.K2_GetRandomReachablePointInRadius` (`self.K2_GetActorLocation` (`|GetArrayItem` (`self.SpawnPoints`) (`KismetMathLibrary.RandomIntegerInRange` 0 (`KismetMathLibrary.Max` (- (`KismetArrayLibrary.Array_Length` (`self.SpawnPoints`)) 1))))) 5000.0 null null))
  (return _randomlocation _returnvalue))

(fn `SpawnAnimals`
  (params (InAnimalClass :type "Actor Class Reference") (MaxSpawnCount :type Integer))
  (locals (Animals :type "Set of /Game/Blueprints/Animals/BP_Animal Object Reference") (SpawnedAnimalCount :type Integer))
  (while (< (`local.SpawnedAnimalCount`) (`local.MaxSpawnCount`))
    (bind (_outspawnablelocation _outfound) (`self.FindSpawnableLocation`))
    (if _outfound
      (bind _returnvalue (`|SpawnActorFromClass` (`local.InAnimalClass`) (`KismetMathLibrary.MakeTransform` _outspawnablelocation) "AdjustIfPossibleButAlwaysSpawn" "MultiplyWithRoot" null null))
      (`/Engine/EditorBlueprintResources/StandardMacros.IsValid` _returnvalue
        (:`Is Valid`
          (bind _asbp_animal (cast `/Game/Blueprints/Animals/BP_Animal` _returnvalue))
          (set `/Game/Blueprints/Animals/BP_Animal.IsMale` (`KismetMathLibrary.RandomBool`) _asbp_animal)
          (`BlueprintSetLibrary.Set_Add` (`local.Animals`) _asbp_animal)
          (`/Engine/EditorBlueprintResources/StandardMacros.IncrementInt` (`local.SpawnedAnimalCount`))))))
  (if (== (`local.InAnimalClass`) "/Game/Blueprints/Animals/Fox/BP_Fox.BP_Fox_C")
    (set `self.Foxes` (`local.Animals`))
    (elif (== (`local.InAnimalClass`) "/Game/Blueprints/Animals/Hare/BP_Hare.BP_Hare_C")
      (set `self.Hares` (`local.Animals`)))))

(fn `SpawnPlants`
  (params (InMaxSpawnCount :type Integer))
  (locals (PlantCount :type Integer))
  (while (and (< (`local.PlantCount`) (`local.InMaxSpawnCount`)) (< (`BlueprintSetLibrary.Set_Length` (`self.Plants`)) (`self.MaxPlantCount`)))
    (bind (_outspawnablelocation _outfound) (`self.FindSpawnableLocation`))
    (if _outfound
      (bind _returnvalue (`|SpawnActorFromClass` "/Game/Blueprints/Plant/BP_Plant.BP_Plant_C" (`KismetMathLibrary.MakeTransform` _outspawnablelocation) "AdjustIfPossibleButAlwaysSpawn" "MultiplyWithRoot" null null))
      (`/Engine/EditorBlueprintResources/StandardMacros.IsValid` _returnvalue
        (:`Is Valid`
          (`BlueprintSetLibrary.Set_Add` (`self.Plants`) _returnvalue)
          (`/Engine/EditorBlueprintResources/StandardMacros.IncrementInt` (`local.PlantCount`)))))))

(fn `UserConstructionScript`)