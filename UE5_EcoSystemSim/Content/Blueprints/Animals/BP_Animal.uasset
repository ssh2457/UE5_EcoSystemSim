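; Animal actor that tracks hunger, thirst and reproduction urge and shows them as bars on a status widget.
; Tick turns the widget toward the player camera, refreshes the bars, and accumulates starving time while hunger is maxed in a specific state.
; IncreseDesire raises each need by its increment, clamped to 0–100, with no caller in this graph.
; Drink resets thirst when the state allows it.
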(event `self.ReceiveTick`
  (params (DeltaSeconds :type "Float (single-precision)"))
  (bind _statuswidget (`self.StatusWidget`))
  (`|ExecutionSequence`
    (:`then_0`
      ; Set GUI
      (`SceneComponent.K2_SetWorldRotation` _statuswidget (`KismetMathLibrary.FindLookAtRotation` (`SceneComponent.K2_GetComponentLocation` _statuswidget) (`SceneComponent.K2_GetComponentLocation` (`PlayerCameraManager.TransformComponent` (`GameplayStatics.GetPlayerCameraManager` 0)))) false false)
      (`self.RefreshUI`))
    (:`then_1`
      ; Update StarvingTime
      (if (`|EnumEquality` (`self.State`) "NewEnumerator1")
        (if (>= (`self.Hunger`) 100)
          (set `self.StarvingTime` (+ DeltaSeconds (`self.StarvingTime`))))))))

(fn `Drink`
  (if (`|EnumEquality` (`self.State`) "NewEnumerator2")
    (set `self.Thirst` 0)
    (`self.RefreshUI`)))

(fn `IncreseDesire`
  (set `self.Hunger` (`KismetMathLibrary.Clamp` (+ (`self.Hunger`) (`self.HungerIncrement`)) 0 100))
  (set `self.Thirst` (`KismetMathLibrary.Clamp` (+ (`self.Thirst`) (`self.ThirstIncrement`)) 0 100))
  (set `self.ReproductionUrge` (`KismetMathLibrary.Clamp` (+ (`self.ReproductionUrge`) (`self.ReproductionUrgeIncrement`)) 0 100)))

(fn `RefreshUI`
  (locals (StatusWidget :type "/Game/Blueprints/Animals/Widgets/WBP_AnimalStatus Object Reference"))
  (bind _aswbp_animal_status (cast `/Game/Blueprints/Animals/Widgets/WBP_AnimalStatus` (`WidgetComponent.GetWidget` (`self.StatusWidget`))))
  (set `local.StatusWidget` _aswbp_animal_status)
  (`|ExecutionSequence`
    (:`then_0`
      ; Update HungerBar
      (`ProgressBar.SetPercent` (`/Game/Blueprints/Animals/Widgets/WBP_AnimalStatus.HungerBar` (`local.StatusWidget`)) (/ (`KismetMathLibrary.Conv_IntToDouble` (`self.Hunger`)) 100.0)))
    (:`then_1`
      ; Update ThirstBar
      (`ProgressBar.SetPercent` (`/Game/Blueprints/Animals/Widgets/WBP_AnimalStatus.ThirstBar` (`local.StatusWidget`)) (/ (`KismetMathLibrary.Conv_IntToDouble` (`self.Thirst`)) 100.0)))
    (:`then_2`
      ; Update ReprodcutionBar
      (`ProgressBar.SetPercent` (`/Game/Blueprints/Animals/Widgets/WBP_AnimalStatus.ReproductionBar` (`local.StatusWidget`)) (/ (`KismetMathLibrary.Conv_IntToDouble` (`self.ReproductionUrge`)) 100.0)))))

(fn `UserConstructionScript`)